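; Pocket (2x2) Rubik's cube actor built from eight mesh components, with animated quarter-turn layer rotations.
; 确定旋转轴 derives axis and direction from hit normal and pitch/yaw input.
; 选择层 gathers cubes sharing the hit cube's position sign on that axis, caching start transforms and rotated targets.
; 执行旋转 plays a timeline that lerps positions linearly while composing an axis-angle rotation onto each starting orientation.
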(event `self.ReceiveBeginPlay`
  (`self.初始化立方体数组`))

(event `self.ReceiveTick`
  (params (DeltaSeconds :type "Float (single-precision)")))

(event `执行旋转`
  (bind (_direction _alpha) (`Timeline|时间轴` :!via `PlayFromStart`)
    (:`Update`
      (for (_array_element _array_index) (`self.选中的方块`)
        (`SceneComponent.K2_SetRelativeTransform` _array_element (`KismetMathLibrary.MakeTransform` (`KismetMathLibrary.VLerp` (`|GetArrayItem` (`self.OldLocatiuon`) _array_index) (`|GetArrayItem` (`self.NewLocatiuon`) _array_index) _alpha) (`KismetMathLibrary.ComposeRotators` (`|GetArrayItem` (`self.OldRotation`) _array_index) (`KismetMathLibrary.RotatorFromAxisAndAngle` (`self.当前旋转轴`) (`KismetMathLibrary.Lerp` 0.0 (`KismetMathLibrary.Conv_IntToDouble` (* (`self.旋转方向`) 90)) _alpha))) (0.99 0.99 0.99)) false false)))))

(fn `UserConstructionScript`
  (`SceneComponent.K2_SetRelativeRotation` :`self` (`self.SpringArm`)))

(fn `保存选中层数据`
  (params (InputPin :type "StaticMeshComponent Object Reference"))
  (bind (_returnvalue_location _returnvalue_rotation) (`KismetMathLibrary.BreakTransform` (`SceneComponent.GetRelativeTransform` InputPin)))
  (`KismetArrayLibrary.Array_AddUnique` (`self.选中的方块`) InputPin)
  (`KismetArrayLibrary.Array_Add` (`self.OldLocatiuon`) _returnvalue_location)
  (`KismetArrayLibrary.Array_Add` (`self.OldRotation`) _returnvalue_rotation)
  (`KismetArrayLibrary.Array_Add` (`self.NewLocatiuon`) (`KismetMathLibrary.RotateAngleAxis` _returnvalue_location (`KismetMathLibrary.Conv_IntToDouble` (* (`self.旋转方向`) 90)) (`self.当前旋转轴`)))
  (`KismetArrayLibrary.Array_Add` (`self.NewRotation`) (`KismetMathLibrary.ComposeRotators` _returnvalue_rotation (`KismetMathLibrary.RotatorFromAxisAndAngle` (`self.当前旋转轴`) 90.0))))

(fn `初始化立方体数组`
  (`KismetArrayLibrary.Array_AddUnique` (`self.所有方块网格体数组`) (`self.Cube000`))
  (`KismetArrayLibrary.Array_AddUnique` (`self.所有方块网格体数组`) (`self.Cube001`))
  (`KismetArrayLibrary.Array_AddUnique` (`self.所有方块网格体数组`) (`self.Cube011`))
  (`KismetArrayLibrary.Array_AddUnique` (`self.所有方块网格体数组`) (`self.Cube100`))
  (`KismetArrayLibrary.Array_AddUnique` (`self.所有方块网格体数组`) (`self.Cube101`))
  (`KismetArrayLibrary.Array_AddUnique` (`self.所有方块网格体数组`) (`self.Cube111`))
  (`KismetArrayLibrary.Array_AddUnique` (`self.所有方块网格体数组`) (`self.Cube010`))
  (`KismetArrayLibrary.Array_AddUnique` (`self.所有方块网格体数组`) (`self.Cube110`)))

(fn `确定旋转轴`
  (params (HitNormal :type "Vector Structure") (Pitch :type "Float (double-precision)") (Yaw :type "Float (double-precision)"))
  (bind (_hitnormal_x _hitnormal_y _hitnormal_z) (`KismetMathLibrary.BreakVector` (`local.HitNormal`)))
  (bind (_hitnormal_x_2 _hitnormal_y_2 _hitnormal_z_2) (`KismetMathLibrary.BreakVector` (`local.HitNormal`)))
  (bind _hitnormal_x_3 (`KismetMathLibrary.BreakVector` (`local.HitNormal`)))
  (bind (_hitnormal_x_4 _hitnormal_y_3) (`KismetMathLibrary.BreakVector` (`local.HitNormal`)))
  (bind _hitnormal_x_5 (`KismetMathLibrary.BreakVector` (`local.HitNormal`)))
  (bind (_hitnormal_x_6 _hitnormal_y_4) (`KismetMathLibrary.BreakVector` (`local.HitNormal`)))
  (bind _returnvalue (`KismetMathLibrary.Abs` _hitnormal_x))
  (bind _returnvalue_2 (`KismetMathLibrary.Abs` _hitnormal_y_2))
  (`KismetSystemLibrary.PrintString` "确定旋转轴")
  (if (and (> _returnvalue (`KismetMathLibrary.Abs` _hitnormal_y)) (> _returnvalue (`KismetMathLibrary.Abs` _hitnormal_z)))
    (`KismetSystemLibrary.PrintString` "法线为X")
    ; 法线为X
    (if (> (`KismetMathLibrary.Abs` (`local.Pitch`)) (`KismetMathLibrary.Abs` (`local.Yaw`)))
      (set `self.当前旋转轴` (0.0 1.0 0.0))
      (if (> _hitnormal_x_3 0.0)
        (if (> (`local.Pitch`) 0.0)
          (set `self.旋转方向` -1)
          (`KismetSystemLibrary.PrintString` "Y轴逆转")
          (else
            (set `self.旋转方向` 1)
            (`KismetSystemLibrary.PrintString` "Y轴正转")))
        (elif (> (`local.Pitch`) 0.0)
          (set `self.旋转方向` 1)
          (`KismetSystemLibrary.PrintString` "Y轴正转")
          (else
            (set `self.旋转方向` -1)
            (`KismetSystemLibrary.PrintString` "Y轴逆转"))))
      (else
        (set `self.当前旋转轴` (0.0 0.0 1.0))
        (if (> _hitnormal_x_5 0.0)
          (if (> 0.0 (`local.Yaw`))
            (set `self.旋转方向` 1)
            (`KismetSystemLibrary.PrintString` "Z轴逆转")
            (else
              (set `self.旋转方向` -1)
              (`KismetSystemLibrary.PrintString` "Z轴正转")))
          (elif (> 0.0 (`local.Yaw`))
            (set `self.旋转方向` 1)
            (`KismetSystemLibrary.PrintString` "Z轴逆转")
            (else
              (set `self.旋转方向` -1)
              (`KismetSystemLibrary.PrintString` "Z轴正转"))))))
    (elif (and (> _returnvalue_2 (`KismetMathLibrary.Abs` _hitnormal_x_2)) (> _returnvalue_2 (`KismetMathLibrary.Abs` _hitnormal_z_2)))
      (`KismetSystemLibrary.PrintString` "法线为Y")
      ; 法线为Y
      (if (> (`KismetMathLibrary.Abs` (`local.Pitch`)) (`KismetMathLibrary.Abs` (`local.Yaw`)))
        (set `self.当前旋转轴` (1.0 0.0 0.0))
        (if (> _hitnormal_y_3 0.0)
          (if (> (`local.Pitch`) 0.0)
            (set `self.旋转方向` 1)
            (`KismetSystemLibrary.PrintString` "X轴逆转")
            (else
              (set `self.旋转方向` -1)
              (`KismetSystemLibrary.PrintString` "X轴正转")))
          (elif (> (`local.Pitch`) 0.0)
            (set `self.旋转方向` -1)
            (`KismetSystemLibrary.PrintString` "X轴正转")
            (else
              (set `self.旋转方向` 1)
              (`KismetSystemLibrary.PrintString` "X轴逆转"))))
        (else
          (set `self.当前旋转轴` (0.0 0.0 1.0))
          (if (> _hitnormal_y_4 0.0)
            (if (> 0.0 (`local.Yaw`))
              (set `self.旋转方向` 1)
              (`KismetSystemLibrary.PrintString` "Z轴正转")
              (else
                (set `self.旋转方向` -1)
                (`KismetSystemLibrary.PrintString` "Z轴逆转")))
            (elif (> 0.0 (`local.Yaw`))
              (set `self.旋转方向` 1)
              (`KismetSystemLibrary.PrintString` "Z轴正转")
              (else
                (set `self.旋转方向` -1)
                (`KismetSystemLibrary.PrintString` "Z轴逆转"))))))
      (else
        (`KismetSystemLibrary.PrintString` "法线为Z")
        ; 法线为Z
        (set `self.当前旋转轴` (0.0 0.0 1.0))
        (if (> (`local.Yaw`) 0.0)
          (set `self.旋转方向` -1)
          (`KismetSystemLibrary.PrintString` "Z轴正转")
          (else
            (set `self.旋转方向` 1)
            (`KismetSystemLibrary.PrintString` "Z轴逆转")))))))

(fn `选择层`
  (params (HitComponent :type "PrimitiveComponent Object Reference"))
  (bind `_当前旋转轴_x` (`KismetMathLibrary.BreakVector` (`self.当前旋转轴`)))
  (bind (`_当前旋转轴_x_2` `_当前旋转轴_y` `_当前旋转轴_z`) (`KismetMathLibrary.BreakVector` (`self.当前旋转轴`)))
  (bind (`_当前旋转轴_x_3` `_当前旋转轴_y_2`) (`KismetMathLibrary.BreakVector` (`self.当前旋转轴`)))
  (bind (_relativelocation_x _relativelocation_y) (`KismetMathLibrary.BreakVector` (`SceneComponent.RelativeLocation` (`local.HitComponent`))))
  (bind (_relativelocation_x_2 _relativelocation_y_2 _relativelocation_z) (`KismetMathLibrary.BreakVector` (`SceneComponent.RelativeLocation` (`local.HitComponent`))))
  (bind _relativelocation_x_3 (`KismetMathLibrary.BreakVector` (`SceneComponent.RelativeLocation` (`local.HitComponent`))))
  ; 清理原有数据
  (`KismetArrayLibrary.Array_Clear` (`self.选中的方块`))
  (`KismetArrayLibrary.Array_Clear` (`self.NewLocatiuon`))
  (`KismetArrayLibrary.Array_Clear` (`self.NewRotation`))
  (`KismetArrayLibrary.Array_Clear` (`self.OldLocatiuon`))
  (`KismetArrayLibrary.Array_Clear` (`self.OldRotation`))
  (`KismetSystemLibrary.PrintString` "旋转一次" true true (struct :`R` 1.0 :`B` 0.0676 :`A` 1.0))
  (if (> `_当前旋转轴_z` 0.0)
    (if (> _relativelocation_z 0.0)
      (for _array_element (`self.所有方块网格体数组`)
        (bind (_relativelocation_x_4 _relativelocation_y_3 _relativelocation_z_2) (`KismetMathLibrary.BreakVector` (`SceneComponent.RelativeLocation` _array_element)))
        (if (> _relativelocation_z_2 0.0)
          (`self.保存选中层数据` _array_element)))
      (else
        (for _array_element_2 (`self.所有方块网格体数组`)
          (bind (_relativelocation_x_5 _relativelocation_y_4 _relativelocation_z_3) (`KismetMathLibrary.BreakVector` (`SceneComponent.RelativeLocation` _array_element_2)))
          (if (< _relativelocation_z_3 0.0)
            (`self.保存选中层数据` _array_element_2)))))
    (elif (> `_当前旋转轴_y_2` 0.0)
      (if (> _relativelocation_y 0.0)
        (for _array_element_3 (`self.所有方块网格体数组`)
          (bind (_relativelocation_x_6 _relativelocation_y_5) (`KismetMathLibrary.BreakVector` (`SceneComponent.RelativeLocation` _array_element_3)))
          (if (> _relativelocation_y_5 0.0)
            (`self.保存选中层数据` _array_element_3)))
        (else
          (for _array_element_4 (`self.所有方块网格体数组`)
            (bind (_relativelocation_x_7 _relativelocation_y_6) (`KismetMathLibrary.BreakVector` (`SceneComponent.RelativeLocation` _array_element_4)))
            (if (< _relativelocation_y_6 0.0)
              (`self.保存选中层数据` _array_element_4)))))
      (elif (> `_当前旋转轴_x` 0.0)
        (if (> _relativelocation_x_3 0.0)
          (for _array_element_5 (`self.所有方块网格体数组`)
            (bind _relativelocation_x_8 (`KismetMathLibrary.BreakVector` (`SceneComponent.RelativeLocation` _array_element_5)))
            (if (> _relativelocation_x_8 0.0)
              (`self.保存选中层数据` _array_element_5)))
          (else
            (for _array_element_6 (`self.所有方块网格体数组`)
              (bind _relativelocation_x_9 (`KismetMathLibrary.BreakVector` (`SceneComponent.RelativeLocation` _array_element_6)))
              (if (< _relativelocation_x_9 0.0)
                (`self.保存选中层数据` _array_element_6)))))))))