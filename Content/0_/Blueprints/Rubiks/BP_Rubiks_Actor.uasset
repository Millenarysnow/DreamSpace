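; A 2x2x2 Rubik's cube actor built from eight fragments whose layers turn in animated quarter turns.
; 确定旋转轴 derives axis and direction from hit normal, dominant pitch/yaw input and, for Z faces, hit piece position.
; 选择层 caches transforms of pieces on the hit side, which 执行旋转 interpolates by timeline.
; 玩家旋转 uses a second timeline to carry a player around the same axis.
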(event `self.ReceiveBeginPlay`
  (`self.初始化立方体Actor数组`))

(event `self.ReceiveTick`
  (params (DeltaSeconds :type "Float (single-precision)")))

(event `执行旋转`
  (bind (_direction _alpha) (`Timeline|时间轴` :!via `PlayFromStart`)
    (:`Update`
      (for (_array_element _array_index) (`self.选中的方块Actor`)
        (bind _output (`|GetArrayItem` (`self.OldLocatiuon`) _array_index))
        (`SceneComponent.K2_SetRelativeTransform` _array_element (`KismetMathLibrary.MakeTransform` (`KismetMathLibrary.VLerp` _output (`KismetMathLibrary.RotateAngleAxis` _output (`KismetMathLibrary.Conv_IntToDouble` (* (`self.旋转方向`) 90)) (`self.当前旋转轴`)) _alpha) (`KismetMathLibrary.ComposeRotators` (`|GetArrayItem` (`self.OldRotation`) _array_index) (`KismetMathLibrary.RotatorFromAxisAndAngle` (`self.当前旋转轴`) (`KismetMathLibrary.Lerp` 0.0 (`KismetMathLibrary.Conv_IntToDouble` (* (`self.旋转方向`) 90)) _alpha))) (0.99 0.99 0.99)) false false)))
    (:`Finished`
      (set `self.IsRotating` false))))

(event `玩家旋转`
  (params (Player :type "/Game/0_/Character/BP_ThirdPersonCharacter Object Reference"))
  ;[0.15 0.006874 0 0.5] 变换玩家相对于魔方的位置变换
  (bind _relativelocation (`self.获取Actor的相对位置` Player))
  (bind (_direction _alpha) (`Timeline|时间轴_0` :!via `PlayFromStart`)
    (:`Update`
      (`self.K2_SetActorLocationAndRotation` Player (+ (`KismetMathLibrary.VLerp` _relativelocation (`KismetMathLibrary.RotateAngleAxis` _relativelocation (`KismetMathLibrary.Conv_IntToDouble` (* (`self.旋转方向`) 90)) (`self.当前旋转轴`)) _alpha) (`self.K2_GetActorLocation`)) (`KismetMathLibrary.ComposeRotators` (`KismetMathLibrary.ComposeRotators` (`|GetArrayItem` (`self.OldRotation`)) (`KismetMathLibrary.RotatorFromAxisAndAngle` (`self.当前旋转轴`) (`KismetMathLibrary.Lerp` 0.0 (`KismetMathLibrary.Conv_IntToDouble` (* (`self.旋转方向`) 90)) _alpha))) (`self.K2_GetActorRotation`)) false false))))

(fn `UserConstructionScript`
  (`SceneComponent.K2_SetRelativeRotation` :`self` (`self.SpringArm`))
  (`self.初始化Actor位置`)
  (`/Game/0_/Blueprints/Rubiks/CubeFragment/CubeFragment.Init` (`self.CubeFragment`)))

(fn `保存选中层数据`
  (params (Actor :type "ChildActorComponent Object Reference"))
  (bind (_returnvalue_location _returnvalue_rotation) (`KismetMathLibrary.BreakTransform` (`SceneComponent.GetRelativeTransform` Actor)))
  (`KismetArrayLibrary.Array_AddUnique` (`self.选中的方块Actor`) Actor)
  (`KismetArrayLibrary.Array_Add` (`self.OldLocatiuon`) _returnvalue_location)
  (`KismetArrayLibrary.Array_Add` (`self.OldRotation`) _returnvalue_rotation))

(fn `初始化Actor位置`
  (`SceneComponent.K2_SetRelativeLocation` (`self.CubeFragment_110`) (50.0 50.0 -50.0) false false)
  (`SceneComponent.K2_SetRelativeLocation` (`self.CubeFragment_111`) (50.0 50.0 50.0) false false)
  (`SceneComponent.K2_SetRelativeLocation` (`self.CubeFragment_101`) (50.0 -50.0 50.0) false false)
  (`SceneComponent.K2_SetRelativeLocation` (`self.CubeFragment_100`) (50.0 -50.0 -50.0) false false)
  (`SceneComponent.K2_SetRelativeLocation` (`self.CubeFragment_000`) (-50.0 -50.0 -50.0) false false)
  (`SceneComponent.K2_SetRelativeLocation` (`self.CubeFragment_001`) (-50.0 -50.0 50.0) false false)
  (`SceneComponent.K2_SetRelativeLocation` (`self.CubeFragment_011`) (-50.0 50.0 50.0) false false)
  (`SceneComponent.K2_SetRelativeLocation` (`self.CubeFragment_010`) (-50.0 50.0 -50.0) false false))

(fn `初始化立方体Actor数组`
  (`KismetArrayLibrary.Array_AddUnique` (`self.所有方块Actor`) (`self.CubeFragment_101`))
  (`KismetArrayLibrary.Array_AddUnique` (`self.所有方块Actor`) (`self.CubeFragment_110`))
  (`KismetArrayLibrary.Array_AddUnique` (`self.所有方块Actor`) (`self.CubeFragment_111`))
  (`KismetArrayLibrary.Array_AddUnique` (`self.所有方块Actor`) (`self.CubeFragment_100`))
  (`KismetArrayLibrary.Array_AddUnique` (`self.所有方块Actor`) (`self.CubeFragment_000`))
  (`KismetArrayLibrary.Array_AddUnique` (`self.所有方块Actor`) (`self.CubeFragment_001`))
  (`KismetArrayLibrary.Array_AddUnique` (`self.所有方块Actor`) (`self.CubeFragment_010`))
  (`KismetArrayLibrary.Array_AddUnique` (`self.所有方块Actor`) (`self.CubeFragment_011`)))

(fn `确定旋转轴`
  (params (HitNormal :type "Vector Structure") (Pitch :type "Float (double-precision)") (Yaw :type "Float (double-precision)") (HitActorRelativeLocatiuon :type "Vector Structure"))
  (bind (_hitnormal_x _hitnormal_y _hitnormal_z) (`KismetMathLibrary.BreakVector` (`local.HitNormal`)))
  (bind (_hitnormal_x_2 _hitnormal_y_2 _hitnormal_z_2) (`KismetMathLibrary.BreakVector` (`local.HitNormal`)))
  (bind _hitnormal_x_3 (`KismetMathLibrary.BreakVector` (`local.HitNormal`)))
  (bind (_hitnormal_x_4 _hitnormal_y_3) (`KismetMathLibrary.BreakVector` (`local.HitNormal`)))
  (bind (_hitactorrelativelocatiuon_x _hitactorrelativelocatiuon_y) (`KismetMathLibrary.BreakVector` (`local.HitActorRelativeLocatiuon`)))
  (bind (_hitactorrelativelocatiuon_x_2 _hitactorrelativelocatiuon_y_2) (`KismetMathLibrary.BreakVector` (`local.HitActorRelativeLocatiuon`)))
  (bind _hitactorrelativelocatiuon_x_3 (`KismetMathLibrary.BreakVector` (`local.HitActorRelativeLocatiuon`)))
  (bind _hitnormal_x_5 (`KismetMathLibrary.BreakVector` (`local.HitNormal`)))
  (bind (_hitnormal_x_6 _hitnormal_y_4) (`KismetMathLibrary.BreakVector` (`local.HitNormal`)))
  (bind _returnvalue (`KismetMathLibrary.Abs` _hitnormal_x))
  (bind _returnvalue_2 (`KismetMathLibrary.Abs` _hitnormal_y_2))
  (if (and (> _returnvalue (`KismetMathLibrary.Abs` _hitnormal_y)) (> _returnvalue (`KismetMathLibrary.Abs` _hitnormal_z)))
    (`KismetSystemLibrary.PrintString` "法线为X")
    ; 法线为X
    (if (> (`KismetMathLibrary.Abs` (`local.Pitch`)) (`KismetMathLibrary.Abs` (`local.Yaw`)))
      (set `self.当前旋转轴` (0.0 1.0 0.0))
      (if (> _hitnormal_x_3 0.0)
        (if (> (`local.Pitch`) 0.0)
          (set `self.旋转方向` -1)
          (`KismetSystemLibrary.PrintString` "Y轴逆转")
          (else
            (set `self.旋转方向` 1)
            (`KismetSystemLibrary.PrintString` "Y轴正转")))
        (elif (> (`local.Pitch`) 0.0)
          (set `self.旋转方向` 1)
          (`KismetSystemLibrary.PrintString` "Y轴正转")
          (else
            (set `self.旋转方向` -1)
            (`KismetSystemLibrary.PrintString` "Y轴逆转"))))
      (else
        (set `self.当前旋转轴` (0.0 0.0 1.0))
        (if (> _hitnormal_x_5 0.0)
          (if (> 0.0 (`local.Yaw`))
            (set `self.旋转方向` 1)
            (`KismetSystemLibrary.PrintString` "Z轴逆转")
            (else
              (set `self.旋转方向` -1)
              (`KismetSystemLibrary.PrintString` "Z轴正转")))
          (elif (> 0.0 (`local.Yaw`))
            (set `self.旋转方向` 1)
            (`KismetSystemLibrary.PrintString` "Z轴逆转")
            (else
              (set `self.旋转方向` -1)
              (`KismetSystemLibrary.PrintString` "Z轴正转"))))))
    (elif (and (> _returnvalue_2 (`KismetMathLibrary.Abs` _hitnormal_x_2)) (> _returnvalue_2 (`KismetMathLibrary.Abs` _hitnormal_z_2)))
      (`KismetSystemLibrary.PrintString` "法线为Y")
      ; 法线为Y
      (if (> (`KismetMathLibrary.Abs` (`local.Pitch`)) (`KismetMathLibrary.Abs` (`local.Yaw`)))
        (set `self.当前旋转轴` (1.0 0.0 0.0))
        (if (> _hitnormal_y_3 0.0)
          (if (> (`local.Pitch`) 0.0)
            (set `self.旋转方向` 1)
            (`KismetSystemLibrary.PrintString` "X轴逆转")
            (else
              (set `self.旋转方向` -1)
              (`KismetSystemLibrary.PrintString` "X轴正转")))
          (elif (> (`local.Pitch`) 0.0)
            (set `self.旋转方向` -1)
            (`KismetSystemLibrary.PrintString` "X轴正转")
            (else
              (set `self.旋转方向` 1)
              (`KismetSystemLibrary.PrintString` "X轴逆转"))))
        (else
          (set `self.当前旋转轴` (0.0 0.0 1.0))
          (if (> _hitnormal_y_4 0.0)
            (if (> 0.0 (`local.Yaw`))
              (set `self.旋转方向` 1)
              (`KismetSystemLibrary.PrintString` "Z轴正转")
              (else
                (set `self.旋转方向` -1)
                (`KismetSystemLibrary.PrintString` "Z轴逆转")))
            (elif (> 0.0 (`local.Yaw`))
              (set `self.旋转方向` 1)
              (`KismetSystemLibrary.PrintString` "Z轴正转")
              (else
                (set `self.旋转方向` -1)
                (`KismetSystemLibrary.PrintString` "Z轴逆转"))))))
      (else
        ; 法线为Z
        (`KismetSystemLibrary.PrintString` "法线为Z")
        (if (< (`KismetMathLibrary.Abs` (`local.Pitch`)) (`KismetMathLibrary.Abs` (`local.Yaw`)))
          (set `self.当前旋转轴` (0.0 0.0 1.0))
          (if (> (`local.Yaw`) 0.0)
            (set `self.旋转方向` -1)
            (`KismetSystemLibrary.PrintString` "Z轴正转")
            (else
              (set `self.旋转方向` 1)
              (`KismetSystemLibrary.PrintString` "Z轴逆转")))
          (elif (> (* _hitactorrelativelocatiuon_x_2 _hitactorrelativelocatiuon_y_2) 0.0)
            ;; 同号
            (if (> _hitactorrelativelocatiuon_x_3 0.0)
              ;; 都大于0
              (if (> (`local.Yaw`) 0.0)
                (if (> (`local.Pitch`) 0.0)
                  (set `self.当前旋转轴` (1.0 0.0 0.0))
                  (set `self.旋转方向` 1)
                  (`KismetSystemLibrary.PrintString` "X轴正转")
                  (else
                    (set `self.当前旋转轴` (0.0 1.0 0.0))
                    (set `self.旋转方向` 1)
                    (`KismetSystemLibrary.PrintString` "Y轴正转")))
                (elif (> (`local.Pitch`) 0.0)
                  (set `self.当前旋转轴` (0.0 1.0 0.0))
                  (set `self.旋转方向` -1)
                  (`KismetSystemLibrary.PrintString` "Y轴逆转")
                  (else
                    (set `self.当前旋转轴` (1.0 0.0 0.0))
                    (set `self.旋转方向` -1)
                    (`KismetSystemLibrary.PrintString` "X轴逆转"))))
              (else
                ;; 都小于0
                (if (> (`local.Yaw`) 0.0)
                  (if (> (`local.Pitch`) 0.0)
                    (set `self.当前旋转轴` (1.0 0.0 0.0))
                    (set `self.旋转方向` -1)
                    (`KismetSystemLibrary.PrintString` "X轴逆转")
                    (else
                      (set `self.当前旋转轴` (0.0 1.0 0.0))
                      (set `self.旋转方向` -1)
                      (`KismetSystemLibrary.PrintString` "Y轴逆转")))
                  (elif (> (`local.Pitch`) 0.0)
                    (set `self.当前旋转轴` (0.0 1.0 0.0))
                    (set `self.旋转方向` 1)
                    (`KismetSystemLibrary.PrintString` "Y轴正转")
                    (else
                      (set `self.当前旋转轴` (1.0 0.0 0.0))
                      (set `self.旋转方向` 1)
                      (`KismetSystemLibrary.PrintString` "X轴正转"))))))
            (else
              ;; 异号
              (if (> _hitactorrelativelocatiuon_y 0.0)
                ;; X小于0，Y大于0
                (if (> (`local.Yaw`) 0.0)
                  (if (> (`local.Pitch`) 0.0)
                    (set `self.当前旋转轴` (0.0 1.0 0.0))
                    (set `self.旋转方向` 1)
                    (`KismetSystemLibrary.PrintString` "Y轴正转")
                    (else
                      (set `self.当前旋转轴` (1.0 0.0 0.0))
                      (set `self.旋转方向` -1)
                      (`KismetSystemLibrary.PrintString` "X轴逆转")))
                  (elif (> (`local.Pitch`) 0.0)
                    (set `self.当前旋转轴` (1.0 0.0 0.0))
                    (set `self.旋转方向` 1)
                    (`KismetSystemLibrary.PrintString` "X轴正转")
                    (else
                      (set `self.当前旋转轴` (0.0 1.0 0.0))
                      (set `self.旋转方向` -1)
                      (`KismetSystemLibrary.PrintString` "Y轴逆转"))))
                (else
                  ;; X大于0，Y小于0
                  (if (> (`local.Yaw`) 0.0)
                    (if (> (`local.Pitch`) 0.0)
                      (set `self.当前旋转轴` (0.0 1.0 0.0))
                      (set `self.旋转方向` -1)
                      (`KismetSystemLibrary.PrintString` "Y轴逆转")
                      (else
                        (set `self.当前旋转轴` (1.0 0.0 0.0))
                        (set `self.旋转方向` 1)
                        (`KismetSystemLibrary.PrintString` "X轴正转")))
                    (elif (> (`local.Pitch`) 0.0)
                      (set `self.当前旋转轴` (1.0 0.0 0.0))
                      (set `self.旋转方向` -1)
                      (`KismetSystemLibrary.PrintString` "X轴逆转")
                      (else
                        (set `self.当前旋转轴` (0.0 1.0 0.0))
                        (set `self.旋转方向` 1)
                        (`KismetSystemLibrary.PrintString` "Y轴正转")))))))))))))

(fn `获取Actor的相对位置`
  (params (Actor :type "Actor Object Reference"))
  (returns (RelativeLocation :type "Vector Structure"))
  (return (- (`self.K2_GetActorLocation` Actor) (`self.K2_GetActorLocation`))))

(fn `选择层`
  (params (ActorRelativeLocation :type "Vector Structure"))
  (locals (`子组件的相对位置` :type "Vector Structure" :default (0.0 0.0 0.0)))
  (bind `_当前旋转轴_x` (`KismetMathLibrary.BreakVector` (`self.当前旋转轴`)))
  (bind (`_当前旋转轴_x_2` `_当前旋转轴_y` `_当前旋转轴_z`) (`KismetMathLibrary.BreakVector` (`self.当前旋转轴`)))
  (bind (`_当前旋转轴_x_3` `_当前旋转轴_y_2`) (`KismetMathLibrary.BreakVector` (`self.当前旋转轴`)))
  (bind (`_子组件的相对位置_x` `_子组件的相对位置_y` `_子组件的相对位置_z`) (`KismetMathLibrary.BreakVector` (`local.子组件的相对位置`)))
  (bind (`_子组件的相对位置_x_2` `_子组件的相对位置_y_2`) (`KismetMathLibrary.BreakVector` (`local.子组件的相对位置`)))
  (bind `_子组件的相对位置_x_3` (`KismetMathLibrary.BreakVector` (`local.子组件的相对位置`)))
  (set `local.子组件的相对位置` ActorRelativeLocation)
  ; 清理原有数据
  (`KismetArrayLibrary.Array_Clear` (`self.选中的方块Actor`))
  (`KismetArrayLibrary.Array_Clear` (`self.OldLocatiuon`))
  (`KismetArrayLibrary.Array_Clear` (`self.OldRotation`))
  (if (> `_当前旋转轴_z` 0.0)
    (if (> `_子组件的相对位置_z` 0.0)
      (for _array_element (`self.所有方块Actor`)
        (bind (_relativelocation_x _relativelocation_y _relativelocation_z) (`KismetMathLibrary.BreakVector` (`SceneComponent.RelativeLocation` _array_element)))
        (if (> _relativelocation_z 0.0)
          (`self.保存选中层数据` _array_element)))
      (else
        (for _array_element_2 (`self.所有方块Actor`)
          (bind (_relativelocation_x_2 _relativelocation_y_2 _relativelocation_z_2) (`KismetMathLibrary.BreakVector` (`SceneComponent.RelativeLocation` _array_element_2)))
          (if (< _relativelocation_z_2 0.0)
            (`self.保存选中层数据` _array_element_2)))))
    (elif (> `_当前旋转轴_y_2` 0.0)
      (if (> `_子组件的相对位置_y_2` 0.0)
        (for _array_element_3 (`self.所有方块Actor`)
          (bind (_relativelocation_x_3 _relativelocation_y_3) (`KismetMathLibrary.BreakVector` (`SceneComponent.RelativeLocation` _array_element_3)))
          (if (> _relativelocation_y_3 0.0)
            (`self.保存选中层数据` _array_element_3)))
        (else
          (for _array_element_4 (`self.所有方块Actor`)
            (bind (_relativelocation_x_4 _relativelocation_y_4) (`KismetMathLibrary.BreakVector` (`SceneComponent.RelativeLocation` _array_element_4)))
            (if (< _relativelocation_y_4 0.0)
              (`self.保存选中层数据` _array_element_4)))))
      (elif (> `_当前旋转轴_x` 0.0)
        (if (> `_子组件的相对位置_x_3` 0.0)
          (for _array_element_5 (`self.所有方块Actor`)
            (bind _relativelocation_x_5 (`KismetMathLibrary.BreakVector` (`SceneComponent.RelativeLocation` _array_element_5)))
            (if (> _relativelocation_x_5 0.0)
              (`self.保存选中层数据` _array_element_5)))
          (else
            (for _array_element_6 (`self.所有方块Actor`)
              (bind _relativelocation_x_6 (`KismetMathLibrary.BreakVector` (`SceneComponent.RelativeLocation` _array_element_6)))
              (if (< _relativelocation_x_6 0.0)
                (`self.保存选中层数据` _array_element_6)))))))))